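; Player controller for what appears to be a free-fall game, managing the HUD and per-frame setup of the player character.
; BeginPlay creates the HUD widget and adds it to the player screen.
; Every Tick casts the pawn to PlayerCharacter, reapplies its sphere's physical material override, and writes game time and death count to the HUD.
; Tick also sets the model's anim class to the DrunkRobot AnimBP every frame.
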(event `self.ReceiveBeginPlay`
  (bind _returnvalue (`|CreateWidget` "/Game/Blueprints/HUD.HUD_C" self))
  (bind _output_get (set `self.HUD` _returnvalue))
  (`UserWidget.AddToPlayerScreen` _output_get 0))

(event `self.ReceiveTick`
  (params (DeltaSeconds :type "Float (single-precision)"))
  (bind _hud (`self.HUD`))
  (`|ExecutionSequence`
    (:`then_0`
      (bind _asplayer_character (cast `PlayerCharacter` (`GameplayStatics.GetPlayerPawn` 0)))
      (`PrimitiveComponent.SetPhysMaterialOverride` (`PlayerCharacter.SphereComponent` _asplayer_character) "/Game/PlayerPhysMat.PlayerPhysMat")
      (`TextBlock.SetText` (`/Game/Blueprints/HUD.timer` _hud) (`KismetTextLibrary.Conv_DoubleToText` (`KismetSystemLibrary.GetGameTimeInSeconds`) "HalfToEven"))
      (`TextBlock.SetText` (`/Game/Blueprints/HUD.death_count` _hud) (`KismetTextLibrary.Conv_IntToText` (`PlayerCharacter.DeathCount` _asplayer_character))))
    (:`then_1`
      (`SkeletalMeshComponent.SetAnimInstanceClass` (`PlayerCharacter.Model` _asplayer_character) "/Game/Models/Player/DrunkRobot_AnimBP.DrunkRobot_AnimBP_C"))))

(fn `UserConstructionScript`)