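; Portal actor that teleports an overlapping PlayerCharacter to its linked Exit portal, unless it is marked as a one-way exit.
; The destination's collision is disabled before teleporting, and each portal's Tick restores its own collision after a short delay, preventing immediate re-entry.
; Optional momentum redirection re-enables the jetpack and passes either the inverted physics velocity or the exit's direction vector to the player.
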(event `self.ReceiveActorBeginOverlap`
  (params (OtherActor :type "Actor Object Reference"))
  (bind _exit (`self.Exit`))
  (`/Engine/EditorBlueprintResources/StandardMacros.IsValid` (`GameplayStatics.GetPlayerPawn` 0)
    (:`Is Valid`
      (if (not (`self.IsOneWayExit`))
        (`/Engine/EditorBlueprintResources/StandardMacros.IsValid` (`self.Exit`)
          (:`Is Valid`
            (bind _asplayer_character (cast `PlayerCharacter` OtherActor))
            (`PrimitiveComponent.SetCollisionEnabled` (`/Game/Blueprints/Portal.Collision` _exit) "NoCollision")
            (`PlayerCharacter.Teleport` _asplayer_character (`self.K2_GetActorLocation` _exit))
            (if (`self.RedirectMomentum`)
              (set `PlayerCharacter.CanUseJetpack` true _asplayer_character)
              (if (`self.InvertMomentum`)
                (bind _returnvalue (`PrimitiveComponent.GetPhysicsLinearVelocity` (`PlayerCharacter.SphereComponent` _asplayer_character) "None"))
                (`PlayerCharacter.RedirectMomemtum` _asplayer_character (* _returnvalue -1.0))
                (else
                  (`PlayerCharacter.RedirectMomemtum` _asplayer_character (`SceneComponent.GetForwardVector` (`/Game/Blueprints/Portal.ExitDirection` _exit))))))))))))

(event `self.ReceiveTick`
  (params (DeltaSeconds :type "Float (single-precision)"))
  (if (`|EnumEquality` (`PrimitiveComponent.GetCollisionEnabled` (`self.Collision`)) "NoCollision")
    (`KismetSystemLibrary.Delay` 1.0)
    (`PrimitiveComponent.SetCollisionEnabled` (`self.Collision`) "QueryAndPhysics")))

(fn `UserConstructionScript`)