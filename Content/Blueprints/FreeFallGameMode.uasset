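; FreeFallGameMode is a game mode that persists running totals of deaths and time across sessions through a savegame object.
; The construction script zeroes both totals, and BeginPlay overwrites them from "slot1" if a save exists.
; The existence check queries an empty slot name rather than "slot1".
; EndPlay creates a new save object, copies both totals into it and writes it to "slot1".
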(event `self.ReceiveBeginPlay`
  (bind _returnvalue (`GameplayStatics.DoesSaveGameExist` ""))
  (if _returnvalue
    (bind _returnvalue_2 (`GameplayStatics.LoadGameFromSlot` "slot1"))
    (bind _assavegame (cast `/Game/Blueprints/savegame` _returnvalue_2))
    (set `self.sum_of_deaths` (`/Game/Blueprints/savegame.sum_death` _assavegame))
    (set `self.sum_of_times` (`/Game/Blueprints/savegame.sum_time` _assavegame))))

(event `self.ReceiveEndPlay`
  (params (EndPlayReason :type "EEndPlayReason Enum" :default "Destroyed"))
  (bind _returnvalue (`GameplayStatics.CreateSaveGameObject` "/Game/Blueprints/savegame.savegame_C"))
  (bind _assavegame (cast `/Game/Blueprints/savegame` _returnvalue))
  (bind _output_get (set `self.save_game` _assavegame))
  (set `/Game/Blueprints/savegame.sum_time` (`self.sum_of_times`) _output_get)
  (set `/Game/Blueprints/savegame.sum_death` (`self.sum_of_deaths`) _output_get)
  (`GameplayStatics.SaveGameToSlot` _output_get "slot1"))

(fn `UserConstructionScript`
  (set `self.sum_of_deaths` 0)
  (set `self.sum_of_times` 0.0))